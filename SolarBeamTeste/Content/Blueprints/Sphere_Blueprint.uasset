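; Sphere actor Blueprint that sets its own world location every tick from sine and cosine of Translate over RotVelocity.
; Translate is multiplied by delta time each tick rather than accumulated, and only the X term gets the large radius scale, with Z fixed at zero.
; A Rotacao function applies local yaw scaled to a day's length in seconds by RotVelocity, but its call is disconnected and never runs.
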(event EventBeginPlay)

(event Collision|EventActorBeginOverlap
  (params (OtherActor :type Actor%20Object%20Reference)))

(event EventTick
  (params (DeltaSeconds :type Float%20%28single-precision%29))
  (bind _output_get (Variables|Default|Settranslate (* DeltaSeconds (Variables|Default|Gettranslate))))
  (Transformation|SetActorLocation (Math|Vector|MakeVector (* (Math|Trig|Sin(Radians) (/ _output_get (Variables|Default|GetrotVelocity))) 5e+03) (Math|Trig|Cos(Radians) (/ _output_get (Variables|Default|GetrotVelocity))) 0.0) false false))

(fn ConstructionScript)