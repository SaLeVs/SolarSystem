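; Planet actor that spins on its own axis while moving in a circular orbit around the world origin.
; Each Tick, Rotacao adds local yaw scaled by DeltaSeconds, Velocity and RotationTime.
; Tick then accumulates time in Translate and sets the location on the XY plane with sine and cosine, using Distance as radius.
; Velocity scales both motions, while TranslationTime sets the orbital rate.
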(event EventBeginPlay)

(event Collision|EventActorBeginOverlap
  (params (OtherActor :type Actor%20Object%20Reference)))

(event EventTick
  (params (DeltaSeconds :type Float%20%28single-precision%29))
  (bind _distance (Variables|Default|Getdistance))
  (Utilities|FlowControl|Sequence
    (:then_0
      (|Rotacao DeltaSeconds))
    (:then_1
      (bind _output_get (Variables|Default|Settranslate (+ DeltaSeconds (Variables|Default|Gettranslate))))
      (Transformation|SetActorLocation (Math|Vector|MakeVector (* (Math|Trig|Sin(Radians) (/ (* _output_get (Variables|Default|Getvelocity)) (Variables|Default|GettranslationTime))) _distance) (* _distance (Math|Trig|Cos(Radians) (/ (* _output_get (Variables|Default|Getvelocity)) (Variables|Default|GettranslationTime)))) 0.0) false false))))

(fn ConstructionScript)